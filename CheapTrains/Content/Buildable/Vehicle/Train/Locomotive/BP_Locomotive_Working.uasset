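; Satisfactory locomotive Blueprint (Cheap Trains) adding name text, toggleable spotlights and Christmas-event decorations.
; Name updates and the Flashlight input call server functions on CheapTrainsRCO, while OnRep functions refresh text and light visibility.
; BeginPlay saves component relative transforms for re-attachment on rerail.
; Rerail gives every child the first saved transform (the root's), and its incrementing Index is never reset here.
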(event EventBeginPlay
  (bind _self self)
  (bind _xmas (Variables|Default|GetXmas))
  (bind _returnvalue (Class|FGEventSubsystem|GetEventSubsystem _self))
  (|CallParentFunction)
  (Utilities|IsValid _returnvalue
    (:Is%20Valid
      (for _array_element (Class|FGEventSubsystem|GetCurrentEvents _returnvalue)
        (switch Utilities|FlowControl|Switch|SwitchonEEvents _array_element
          (:EV_None
            (Rendering|SetVisibility _xmas false true :!label _label)
            (Development|SetHiddeninGame _xmas true false))
          (:EV_Christmas
            (Rendering|SetVisibility _xmas true true)
            (Development|SetHiddeninGame _xmas false true))
          (:EV_Birthday
            (goto _label))
          (:EV_CSSBirthday
            (goto _label))
          (:EV_FirstOfApril
            (goto _label)))))
    (:Is%20Not%20Valid
      _))
  (CallFunction|OnStartProgTrainsSaveMeshPositions)
  (bind _returnvalue_2 (Class|CheapTrainsLibrary|GetRCO "/CheapTrains/CheapTrainsRCO.CheapTrainsRCO_C"))
  (bind _ascheap_trains_rco (Utilities|Casting|CastToCheapTrainsRCO _returnvalue_2))
  (Default|ServerUpdateTrainName _ascheap_trains_rco self (Class|FGTrain|GetTrainName (Class|FGRailroadVehicle|GetTrain))))

(event Collision|EventActorBeginOverlap
  (params (OtherActor :type Actor%20Object%20Reference))
  (|CallParentFunction OtherActor) ; This node is disabled and will not be called.\nDrag off pins to build functionality.
)

(event EventOnVehicleStartup
  (bind _returnvalue (Class|CheapTrainsLibrary|GetRCO "/CheapTrains/CheapTrainsRCO.CheapTrainsRCO_C"))
  (bind _ascheap_trains_rco (Utilities|Casting|CastToCheapTrainsRCO _returnvalue))
  (Default|ServerUpdateTrainName _ascheap_trains_rco self (Class|FGTrain|GetTrainName (Class|FGRailroadVehicle|GetTrain))))

(event EventOnNameChanged
  (bind _returnvalue (Class|CheapTrainsLibrary|GetRCO "/CheapTrains/CheapTrainsRCO.CheapTrainsRCO_C"))
  (bind _ascheap_trains_rco (Utilities|Casting|CastToCheapTrainsRCO _returnvalue))
  (Default|ServerUpdateTrainName _ascheap_trains_rco self (Class|FGTrain|GetTrainName (Class|FGRailroadVehicle|GetTrain))))

(event EventTick
  (params (DeltaSeconds :type Float%20%28single-precision%29))
  (|CallParentFunction DeltaSeconds))

(event EventUpdateTrainName
  (bind _returnvalue (Class|FGRailroadVehicle|GetTrain))
  (bind _returnvalue_2 (Class|FGTrain|GetTrainName _returnvalue))
  (bind _isserver (CallFunction|IsServer self))
  (if _isserver
    (if (not (Utilities|Enum|Equal(Enum) _returnvalue_2 (Variables|Default|GetTrainName_Prog)))
      (bind _returnvalue_3 (Class|CheapTrainsLibrary|GetRCO "/CheapTrains/CheapTrainsRCO.CheapTrainsRCO_C"))
      (bind _ascheap_trains_rco (Utilities|Casting|CastToCheapTrainsRCO _returnvalue_3))
      (Default|ServerUpdateTrainName _ascheap_trains_rco self _returnvalue_2))))

(event EventOnRerail
  (CallFunction|OnRerailProgTrains))

(event Input|ActionEvents|InputActionFlashlight
  (params (Key :type Key%20Structure :default "None"))
  (:Pressed
    (bind _returnvalue (Class|CheapTrainsLibrary|GetRCO "/CheapTrains/CheapTrainsRCO.CheapTrainsRCO_C"))
    (bind _ascheap_trains_rco (Utilities|Casting|CastToCheapTrainsRCO _returnvalue))
    (Default|ServerToggleTrainLights _ascheap_trains_rco self)))

(fn ConstructionScript
  (|CallParentFunction))

(fn OnRepLightson
  (bind _lightson (Variables|Default|GetLightsOn))
  (Rendering|SetVisibility (Variables|Default|GetSpotLight_1) _lightson false)
  (Rendering|SetVisibility (Variables|Default|GetSpotLight_2) _lightson false))

(fn OnRepTrainNameProg
  (bind _trainname_prog (Variables|Default|GetTrainName_Prog))
  (Rendering|Components|TextRender|SetText (Variables|Default|GetTextRender) _trainname_prog)
  (Rendering|Components|TextRender|SetText (Variables|Default|GetTextRender1) _trainname_prog))

(fn OnRerailProgTrains
  (bind _newdecalsroot (Variables|Default|GetNewDecalsRoot))
  (bind _xmas (Variables|Default|GetXmas))
  (bind _textrender (Variables|Default|GetTextRender))
  (bind _newdecalsroot_2 (Variables|Default|GetNewDecalsRoot))
  (bind _textrender1 (Variables|Default|GetTextRender1))
  (bind _spotlight_1 (Variables|Default|GetSpotLight_1))
  (bind _spotlight_2 (Variables|Default|GetSpotLight_2))
  (Transformation|AttachComponentToComponent _newdecalsroot_2 (Variables|Default|GetmMesh) "Body" "KeepRelative" "KeepRelative" "KeepRelative" true)
  (Transformation|SetRelativeLocationAndRotation _newdecalsroot_2 (Utilities|Array|Get(acopy) (Variables|Default|GetReRail_LocArray) (LocalVariables|Getindex)) (Utilities|Array|Get(acopy) (Variables|Default|GetReRailRotArray) (LocalVariables|Getindex)) false true)
  (bind _output_get (LocalVariables|Setindex (+ (LocalVariables|Getindex) 1)))
  (Transformation|AttachComponentToComponent _xmas _newdecalsroot_2 "None" "KeepRelative" "KeepRelative" "KeepRelative" true)
  (Transformation|SetRelativeLocationAndRotation _xmas (Utilities|Array|Get(acopy) (Variables|Default|GetReRail_LocArray)) (Utilities|Array|Get(acopy) (Variables|Default|GetReRailRotArray)) false true)
  (bind _output_get_2 (LocalVariables|Setindex (+ _output_get 1)))
  (Transformation|AttachComponentToComponent _textrender (Variables|Default|GetNewDecalsRoot) "None" "KeepRelative" "KeepRelative" "KeepRelative" true)
  (Transformation|SetRelativeLocationAndRotation _textrender (Utilities|Array|Get(acopy) (Variables|Default|GetReRail_LocArray)) (Utilities|Array|Get(acopy) (Variables|Default|GetReRailRotArray)) false true)
  (bind _output_get_3 (LocalVariables|Setindex (+ _output_get_2 1)))
  (Transformation|AttachComponentToComponent _textrender1 _newdecalsroot "None" "KeepRelative" "KeepRelative" "KeepRelative" true)
  (Transformation|SetRelativeLocationAndRotation _textrender1 (Utilities|Array|Get(acopy) (Variables|Default|GetReRail_LocArray)) (Utilities|Array|Get(acopy) (Variables|Default|GetReRailRotArray)) false true)
  (bind _output_get_4 (LocalVariables|Setindex (+ _output_get_3 1)))
  (Transformation|AttachComponentToComponent _spotlight_1 (Variables|Default|GetNewDecalsRoot) "None" "KeepRelative" "KeepRelative" "KeepRelative" true)
  (Transformation|SetRelativeLocationAndRotation _spotlight_1 (Utilities|Array|Get(acopy) (Variables|Default|GetReRail_LocArray)) (Utilities|Array|Get(acopy) (Variables|Default|GetReRailRotArray)) false true)
  (bind _output_get_5 (LocalVariables|Setindex (+ _output_get_4 1)))
  (Transformation|AttachComponentToComponent _spotlight_2 _newdecalsroot "None" "KeepRelative" "KeepRelative" "KeepRelative" true)
  (Transformation|SetRelativeLocationAndRotation _spotlight_2 (Utilities|Array|Get(acopy) (Variables|Default|GetReRail_LocArray)) (Utilities|Array|Get(acopy) (Variables|Default|GetReRailRotArray)) false true)
  (LocalVariables|Setindex (+ _output_get_5 1))
  (return))

(fn OnStartProgTrainsSaveMeshPositions
  (bind _newdecalsroot (Variables|Default|GetNewDecalsRoot))
  (bind _xmas (Variables|Default|GetXmas))
  (bind _rerailrotarray (Variables|Default|GetReRailRotArray))
  (bind _textrender (Variables|Default|GetTextRender))
  (bind _textrender1 (Variables|Default|GetTextRender1))
  (bind _spotlight_1 (Variables|Default|GetSpotLight_1))
  (bind _spotlight_2 (Variables|Default|GetSpotLight_2))
  (bind _rerail_locarray (Variables|Default|GetReRail_LocArray))
  (Utilities|Array|Add _rerail_locarray (Variables|/Script/Engine.SceneComponent|GetRelativeLocation _newdecalsroot))
  (Utilities|Array|Add _rerailrotarray (Variables|/Script/Engine.SceneComponent|GetRelativeRotation _newdecalsroot))
  (Utilities|Array|Add _rerail_locarray (Variables|/Script/Engine.SceneComponent|GetRelativeLocation _xmas))
  (Utilities|Array|Add _rerailrotarray (Variables|/Script/Engine.SceneComponent|GetRelativeRotation _xmas))
  (Utilities|Array|Add _rerail_locarray (Variables|/Script/Engine.SceneComponent|GetRelativeLocation _textrender))
  (Utilities|Array|Add _rerailrotarray (Variables|/Script/Engine.SceneComponent|GetRelativeRotation _textrender))
  (Utilities|Array|Add _rerail_locarray (Variables|/Script/Engine.SceneComponent|GetRelativeLocation _textrender1))
  (Utilities|Array|Add _rerailrotarray (Variables|/Script/Engine.SceneComponent|GetRelativeRotation _textrender1))
  (Utilities|Array|Add _rerail_locarray (Variables|/Script/Engine.SceneComponent|GetRelativeLocation _spotlight_1))
  (Utilities|Array|Add _rerailrotarray (Variables|/Script/Engine.SceneComponent|GetRelativeRotation _spotlight_1))
  (Utilities|Array|Add _rerail_locarray (Variables|/Script/Engine.SceneComponent|GetRelativeLocation _spotlight_2))
  (Utilities|Array|Add _rerailrotarray (Variables|/Script/Engine.SceneComponent|GetRelativeRotation _spotlight_2))
  (return))